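; Moving platform that travels along a spline while the golf character overlaps its trigger box.
; Overlap plays the MovePlatform timeline, whose TravelDistance scales the spline length to set the mesh's world location; ending overlap reverses it.
; Mesh rotation always uses the roll and yaw at the spline's start with zero pitch, so the platform does not turn along the path.
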(event OnComponentBeginOverlap(Box)
  (params (OverlappedComponent :type Primitive%20Component%20Object%20Reference) (OtherActor :type Actor%20Object%20Reference) (OtherComp :type Primitive%20Component%20Object%20Reference) (OtherBodyIndex :type Integer) (bFromSweep :type Boolean) (SweepResult :type Hit%20Result%20Structure%20%28by%20ref%29))
  (bind _spline (Variables|Default|GetSpline))
  (bind _returnvalue (Spline|GetRotationatDistanceAlongSpline _spline 0.0 "Local"))
  (Utilities|Casting|CastToGolfGameCharacter OtherActor)
  (bind _traveldistance (Timeline|MovePlatform Play)
    (:Update
      (Transformation|SetWorldLocation (Variables|Default|GetStaticMesh) (Spline|GetLocationatDistanceAlongSpline _spline (* _traveldistance (Spline|GetSplineLength (Variables|Default|GetSpline))) "World") false false)
      (Transformation|SetRelativeRotation (Variables|Default|GetStaticMesh) (Math|Rotator|MakeRotator (.roll _returnvalue) 0.0 (.yaw _returnvalue)) false false))))

(event OnComponentEndOverlap(Box)
  (params (OverlappedComponent :type Primitive%20Component%20Object%20Reference) (OtherActor :type Actor%20Object%20Reference) (OtherComp :type Primitive%20Component%20Object%20Reference) (OtherBodyIndex :type Integer))
  (bind _spline (Variables|Default|GetSpline))
  (bind _returnvalue (Spline|GetRotationatDistanceAlongSpline _spline 0.0 "Local"))
  (Utilities|Casting|CastToGolfGameCharacter OtherActor)
  (bind _traveldistance (Timeline|MovePlatform Reverse)
    (:Update
      (Transformation|SetWorldLocation (Variables|Default|GetStaticMesh) (Spline|GetLocationatDistanceAlongSpline _spline (* _traveldistance (Spline|GetSplineLength (Variables|Default|GetSpline))) "World") false false)
      (Transformation|SetRelativeRotation (Variables|Default|GetStaticMesh) (Math|Rotator|MakeRotator (.roll _returnvalue) 0.0 (.yaw _returnvalue)) false false))))

(event EventBeginPlay
  (bind _spline (Variables|Default|GetSpline))
  (bind _returnvalue (Spline|GetRotationatDistanceAlongSpline _spline 0.0 "Local"))
  (Transformation|SetRelativeRotation (Variables|Default|GetStaticMesh) (Math|Rotator|MakeRotator (.roll _returnvalue) 0.0 (.yaw _returnvalue)) false false))

(fn ConstructionScript)