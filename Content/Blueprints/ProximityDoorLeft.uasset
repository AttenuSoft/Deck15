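; Proximity sliding door, the left one by name, that opens when a GolfGameCharacter enters its Box trigger and closes when it leaves.
; The DoorAnimation timeline drives the mesh's relative location, playing forward on entry and reversing on exit.
; Looping timers re-arm separate open and close flags to throttle the sounds, which play at world origin.
; MoveTrigger lowers the trigger box but is not called within this Blueprint.
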(event OnComponentBeginOverlap(Box)
  (params (OverlappedComponent :type Primitive%20Component%20Object%20Reference) (OtherActor :type Actor%20Object%20Reference) (OtherComp :type Primitive%20Component%20Object%20Reference) (OtherBodyIndex :type Integer) (bFromSweep :type Boolean) (SweepResult :type Hit%20Result%20Structure%20%28by%20ref%29))
  (Utilities|Casting|CastToGolfGameCharacter OtherActor)
  (if (Variables|Default|GetbCanPlayOpenAudio)
    (Audio|PlaySoundatLocation "/Game/Audio/Doors/door_open4_soundcue.door_open4_soundcue" "0, 0, 0" "0, 0, 0" 1.0 1.0 0.0 0 0 0)
    (Variables|Default|SetbCanPlayOpenAudio false)
    (bind _doorslide (Timeline|DoorAnimation Play)
      (:Update
        (Transformation|SetRelativeLocation (Variables|Default|GetDoorMesh) _doorslide false false)))
    (else
      (Timeline|DoorAnimation Play))))

(event OnComponentEndOverlap(Box)
  (params (OverlappedComponent :type Primitive%20Component%20Object%20Reference) (OtherActor :type Actor%20Object%20Reference) (OtherComp :type Primitive%20Component%20Object%20Reference) (OtherBodyIndex :type Integer))
  (Utilities|Casting|CastToGolfGameCharacter OtherActor)
  (if (Variables|Default|GetbCanPlayCloseAudio)
    (Audio|PlaySoundatLocation "/Game/Audio/Doors/door_open3.door_open3" "0, 0, 0" "0, 0, 0" 1.0 1.0 0.0 0 0 0)
    (Variables|Default|SetbCanPlayCloseAudio false)
    (bind _doorslide (Timeline|DoorAnimation Reverse)
      (:Update
        (Transformation|SetRelativeLocation (Variables|Default|GetDoorMesh) _doorslide false false)))
    (else
      (Timeline|DoorAnimation Reverse))))

(event EventBeginPlay
  (Utilities|Time|SetTimerbyFunctionName 0 "SetCanPlayOpenAudio" 0.5 true)
  (Utilities|Time|SetTimerbyFunctionName 0 "SetCanPlayCloseAudio" 0.5 true))

(fn ConstructionScript)

(fn SetCanPlayOpenAudio
  (Variables|Default|SetbCanPlayOpenAudio true))

(fn SetCanPlayCloseAudio
  (Variables|Default|SetbCanPlayCloseAudio true))

(fn MoveTrigger
  (bind _box (Variables|Default|GetBox))
  (Transformation|SetWorldLocation _box (- (Transformation|GetWorldLocation _box) "0, 0,420.000000") false false))