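; Sliding door Blueprint for the golf game, driven by the DoorAnimation timeline, which sets the mesh's relative location.
; A box trigger plays the timeline when a GolfGameCharacter enters and reverses it on exit.
; Tick checks IsBallInGoalDoorTrigger, prints its state for debugging and keeps reversing the timeline while false.
; The file contains no level-loading logic and never sets that flag.
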(event OnComponentBeginOverlap(Box)
  (params (OverlappedComponent :type Primitive%20Component%20Object%20Reference) (OtherActor :type Actor%20Object%20Reference) (OtherComp :type Primitive%20Component%20Object%20Reference) (OtherBodyIndex :type Integer) (bFromSweep :type Boolean) (SweepResult :type Hit%20Result%20Structure%20%28by%20ref%29))
  (Utilities|Casting|CastToGolfGameCharacter OtherActor)
  (bind _doorslide (Timeline|DoorAnimation Play)
    (:Update
      (Transformation|SetRelativeLocation (Variables|Default|GetDoorMesh) _doorslide false false))))

(event OnComponentEndOverlap(Box)
  (params (OverlappedComponent :type Primitive%20Component%20Object%20Reference) (OtherActor :type Actor%20Object%20Reference) (OtherComp :type Primitive%20Component%20Object%20Reference) (OtherBodyIndex :type Integer))
  (Utilities|Casting|CastToGolfGameCharacter OtherActor)
  (bind _doorslide (Timeline|DoorAnimation Reverse)
    (:Update
      (Transformation|SetRelativeLocation (Variables|Default|GetDoorMesh) _doorslide false false))))

(event EventTick
  (params (DeltaSeconds :type Float%20%28single-precision%29))
  (if (Variables|Default|GetIsBallInGoalDoorTrigger)
    (Development|PrintString "DOOR TRUE")
    (else
      (Development|PrintString "DOOR FALSE")
      (bind _doorslide (Timeline|DoorAnimation Reverse)
        (:Update
          (Transformation|SetRelativeLocation (Variables|Default|GetDoorMesh) _doorslide false false))))))

(fn ConstructionScript)