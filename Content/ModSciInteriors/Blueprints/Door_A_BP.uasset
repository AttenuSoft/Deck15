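; Automatic sci-fi door that slides open when something enters its trigger volume and closes when it leaves.
; A timeline lerps the door mesh between closed and open relative positions, playing forward on overlap begin and reversing on end.
; Looping one-second timers re-arm flags that throttle the open and close sounds, which play at world origin.
; Two steam effects fire only alongside the open sound.
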(event OnComponentBeginOverlap(Trigger)
  (params (OverlappedComponent :type Primitive%20Component%20Object%20Reference) (OtherActor :type Actor%20Object%20Reference) (OtherComp :type Primitive%20Component%20Object%20Reference) (OtherBodyIndex :type Integer) (bFromSweep :type Boolean) (SweepResult :type Hit%20Result%20Structure%20%28by%20ref%29))
  (if (Variables|Default|GetbCanPlayOpenAudio)
    (Audio|PlaySoundatLocation "/Game/Audio/Doors/door_open4_soundcue.door_open4_soundcue" "0, 0, 0" "0, 0, 0" 1.0 1.0 0.0 0 0 0)
    (Variables|Default|SetbCanPlayOpenAudio false)
    (Components|Activation|Activate (Variables|Default|GetSteamDoor) false)
    (bind _doorposition (Timeline|Timeline_0 Play)
      (:Update
        (Transformation|SetRelativeLocation (Variables|Default|GetDoor_Small_A) (Math|Vector|Lerp(Vector) (Variables|Door|GetDoorClosed) (Variables|Door|GetDoorOpen) _doorposition) false false)))
    (else
      (Timeline|Timeline_0 Play))))

(event OnComponentEndOverlap(Trigger)
  (params (OverlappedComponent :type Primitive%20Component%20Object%20Reference) (OtherActor :type Actor%20Object%20Reference) (OtherComp :type Primitive%20Component%20Object%20Reference) (OtherBodyIndex :type Integer))
  (if (Variables|Default|GetbCanPLayCloseAudio)
    (Audio|PlaySoundatLocation "/Game/Audio/Doors/door_open3.door_open3" "0, 0, 0" "0, 0, 0" 1.0 1.0 0.0 0 0 0)
    (Variables|Default|SetbCanPLayCloseAudio false)
    (bind _doorposition (Timeline|Timeline_0 Reverse)
      (:Update
        (Transformation|SetRelativeLocation (Variables|Default|GetDoor_Small_A) (Math|Vector|Lerp(Vector) (Variables|Door|GetDoorClosed) (Variables|Door|GetDoorOpen) _doorposition) false false)))
    (else
      (Timeline|Timeline_0 Reverse))))

(event EventBeginPlay
  (Utilities|Time|SetTimerbyFunctionName 0 "SetCanPlayOpenAudio" 1.0 true)
  (Utilities|Time|SetTimerbyFunctionName 0 "SetCanPlayCloseAudio" 1.0 true))

(fn ConstructionScript)

(fn SetCanPlayCloseAudio
  (Variables|Default|SetbCanPLayCloseAudio true))

(fn SetCanPlayOpenAudio
  (Variables|Default|SetbCanPlayOpenAudio true))